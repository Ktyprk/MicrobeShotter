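; BP_MeeleEnemy is a melee enemy that reacts to projectile overlaps.
; It plays the Hit montage on BeginPlay and from a custom event.
; Each projectile overlap briefly swaps the mesh material as a flash, and if Meleehealth is depleted, hides the mesh, spawns steam emitters and destroys the actor after a delay.
; The health decrement is unconnected, so this graph never lowers Meleehealth.
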(event `self.ReceiveBeginPlay`
  (`|PlayMontage` (`self.Mesh`) "/Game/MicrobeShotter/EnemyAI/purpleanimcharacter/hit.hit"))

(event `CustomEvent_0`
  (`|PlayMontage` (`self.Mesh`) "/Game/MicrobeShotter/EnemyAI/purpleanimcharacter/hit.hit"))

(event `self.hiy.OnComponentBeginOverlap`
  (params (OverlappedComponent :type "PrimitiveComponent Object Reference") (OtherActor :type "Actor Object Reference") (OtherComp :type "PrimitiveComponent Object Reference") (OtherBodyIndex :type Integer) (bFromSweep :type Boolean) (SweepResult :type "HitResult Structure (by ref)")))

(event `self.ReceiveActorBeginOverlap`
  (params (OtherActor :type "Actor Object Reference"))
  (cast `/Game/MicrobeShotter/weapon/projectile` OtherActor)
  (`|ExecutionSequence`
    (:`then_0`
      (if (<= (`self.meleehealth`) 0)
        (`/Engine/EditorBlueprintResources/StandardMacros.DoOnce` false
          (:`Completed`
            (`SceneComponent.SetVisibility` (`self.Mesh`) false false)
            (`|ExecutionSequence`
              (:`then_0`
                (bind _returnvalue (`GameplayStatics.SpawnEmitterAtLocation` "/Game/StarterContent/Particles/P_Steam_Lit.P_Steam_Lit" (`self.K2_GetActorLocation`) (struct) (5.0 5.0 5.0))))
              (:`then_1`
                (bind _returnvalue_2 (`GameplayStatics.SpawnEmitterAtLocation` "/Game/StarterContent/Particles/P_Steam_Lit.P_Steam_Lit" (`self.K2_GetActorLocation`) (struct) (5.0 5.0 5.0)))))
            (`KismetSystemLibrary.Delay` 1.0)
            (`ActorComponent.K2_DestroyComponent` _returnvalue)
            (`ActorComponent.K2_DestroyComponent` _returnvalue_2)
            (`self.K2_DestroyActor`)))))
    (:`then_1`
      (`PrimitiveComponent.SetMaterial` (`self.Mesh`) 0 "/Game/MicrobeShotter/Level/HospitalAssets/Hasset3/HASTANEODASI2/Materials/16_Sofa.16_Sofa")
      (`KismetSystemLibrary.Delay` 0.2)
      (`PrimitiveComponent.SetMaterial` (`self.Mesh`) 0 "/Game/MicrobeShotter/EnemyAI/Bacteria/littledemon.littledemon"))))

(fn `UserConstructionScript`)