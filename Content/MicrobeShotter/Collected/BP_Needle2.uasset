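; BP_Needle2 is a collectible needle pickup that adds to the NeedleCount on BP_FPCGameMode.
; BeginPlay caches references to the game mode and the BP_FPC player character.
; When anything begins overlapping its Box, it checks the player's Fartik flag, retrying every 0.2 seconds until true, then increments the count and destroys itself.
; The retry loop never rechecks the overlap, so collection can complete after the overlap ends.
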(event OnComponentBeginOverlap(Box)
  (params (OverlappedComponent :type Primitive%20Component%20Object%20Reference) (OtherActor :type Actor%20Object%20Reference) (OtherComp :type Primitive%20Component%20Object%20Reference) (OtherBodyIndex :type Integer) (bFromSweep :type Boolean) (SweepResult :type Hit%20Result%20Structure%20%28by%20ref%29))
  (bind _as_bp_fpcgame_mode (Variables|Default|GetAs%20BP%20FPCGame%20Mode))
  (if (Variables|/Game/MicrobeShotter/BP_FPC.BP_FPC_C|Getfartik (Variables|Default|GetAs%20BP%20FPC)) :!label _label
    (Variables|/Game/MicrobeShotter/BP_FPCGameMode.BP_FPCGameMode_C|SetNeedleCount _as_bp_fpcgame_mode (+ (Variables|/Game/MicrobeShotter/BP_FPCGameMode.BP_FPCGameMode_C|GetNeedleCount _as_bp_fpcgame_mode) 1))
    (Actor|DestroyActor)
    (else
      (Utilities|FlowControl|Delay 0.2)
      (goto _label))))

(event EventBeginPlay
  (bind _asbp_fpcgame_mode (Utilities|Casting|CastToBP_FPCGameMode (Game|GetGameMode)))
  (Variables|Default|SetAs%20BP%20FPCGame%20Mode _asbp_fpcgame_mode)
  (bind _asbp_fpc (Utilities|Casting|CastToBP_FPC (Game|GetPlayerCharacter 0)))
  (Variables|Default|SetAs%20BP%20FPC _asbp_fpc))

(event Collision|EventActorBeginOverlap
  (params (OtherActor :type Actor%20Object%20Reference)))

(fn ConstructionScript)