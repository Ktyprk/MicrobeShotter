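; BP_needle is a collectible needle pickup that adds to the player's score when touched.
; It caches the BP_FPCGameMode on BeginPlay, and its Sphere overlap sends CollectedNeedleMessage to the overlapping actor, then triggers CollectedNeedle.
; CollectedNeedle adds CountToAdd through the game mode and destroys the actor after a short delay.
; DoOnce gates on both events prevent repeat collection, though the overlap does not filter which actor touched it.
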(event OnComponentBeginOverlap(Sphere)
  (params (OverlappedComponent :type Primitive%20Component%20Object%20Reference) (OtherActor :type Actor%20Object%20Reference) (OtherComp :type Primitive%20Component%20Object%20Reference) (OtherBodyIndex :type Integer) (bFromSweep :type Boolean) (SweepResult :type Hit%20Result%20Structure%20%28by%20ref%29))
  (Utilities|FlowControl|DoOnce false
    (:Completed
      (Class|CollectedNeedleINT|CollectedNeedle(Message) OtherActor)
      (CallFunction|CollectedNeedle))))

(event EventBeginPlay
  (bind _asbp_fpcgame_mode (Utilities|Casting|CastToBP_FPCGameMode (Game|GetGameMode)))
  (Variables|Default|SetGameModeRef _asbp_fpcgame_mode))

(event Collision|EventActorBeginOverlap
  (params (OtherActor :type Actor%20Object%20Reference)))

(event EventTick
  (params (DeltaSeconds :type Float%20%28single-precision%29)))

(event EventCollectedNeedle
  (Utilities|FlowControl|DoOnce false
    (:Completed
      (Default|AddPlayerScore (Variables|Default|GetGameModeRef) (Variables|Default|GetCountToAdd))
      (Utilities|FlowControl|Delay 0.2)
      (Actor|DestroyActor))))

(fn ConstructionScript)